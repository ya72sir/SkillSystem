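; Base enemy character Blueprint that takes typed damage and hurts the player on contact.
; Incoming damage is matched against the enemy's vulnerable and resistant damage type classes, with a macro applying the matching multiplier to Health.
; Each damage and death outcome spawns its own particle effect, and deaths destroy the actor.
; Hits on BP_Player apply AttackDamage, throttled by a DoOnce that resets after a short delay.
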(event `self.ReceiveAnyDamage`
  (params (Damage :type "Float (single-precision)") (DamageType :type "DamageType Object Reference") (InstigatedBy :type "Controller Object Reference") (DamageCauser :type "Actor Object Reference"))
  (bind _returnvalue (`SceneComponent.K2_GetComponentLocation` (`self.CapsuleComponent`)))
  (bind _returnvalue_2 (`SceneComponent.K2_GetComponentLocation` (`self.Mesh`)))
  (bind _returnvalue_3 (`SceneComponent.K2_GetComponentLocation` (`self.Mesh`)))
  (`self.CalculateDamage` Damage DamageType
    (:`VulnerableDeath`
      (`GameplayStatics.SpawnEmitterAtLocation` "/Game/InfinityBladeEffects/Effects/FX_Monsters/FX_Monster_Gruntling/FlameThrower/P_FlameExplode.P_FlameExplode" _returnvalue_2 (struct) (2.0 2.0 2.0))
      (`self.K2_DestroyActor`))
    (:`Vulnerable Damage`
      (`GameplayStatics.SpawnEmitterAtLocation` "/Game/InfinityBladeEffects/Effects/FX_Monsters/FX_Monster_Gruntling/FlameThrower/P_FlameExplode.P_FlameExplode" _returnvalue_2))
    (:`Resistant Death`
      (`GameplayStatics.SpawnEmitterAtLocation` "/Game/InfinityBladeEffects/Effects/FX_Mobile/Lightning/P_LineToPoint_Blast_Lightning_00.P_LineToPoint_Blast_Lightning_00" _returnvalue_3 (struct) (1.5 1.5 1.5))
      (`self.K2_DestroyActor`))
    (:`Resistant Damage`
      (`GameplayStatics.SpawnEmitterAtLocation` "/Game/InfinityBladeEffects/Effects/FX_Mobile/Lightning/P_LineToPoint_Blast_Lightning_00.P_LineToPoint_Blast_Lightning_00" _returnvalue_3 (struct) (0.75 0.75 0.75)))
    (:`Normal Death`
      (`GameplayStatics.SpawnEmitterAtLocation` "/Game/MetroidVania/Library/Particals/P_Explosion.P_Explosion" _returnvalue (struct) (2.0 2.0 2.0))
      (`self.K2_DestroyActor`))
    (:`Normal Damage`
      (`GameplayStatics.SpawnEmitterAtLocation` "/Game/MetroidVania/Library/Particals/P_Explosion.P_Explosion" _returnvalue))))

(event `self.ReceiveHit`
  (params (MyComp :type "PrimitiveComponent Object Reference") (Other :type "Actor Object Reference") (OtherComp :type "PrimitiveComponent Object Reference") (bSelfMoved :type Boolean) (HitLocation :type "Vector Structure") (HitNormal :type "Vector Structure") (NormalImpulse :type "Vector Structure") (Hit :type "HitResult Structure (by ref)"))
  (bind _asbp_player (cast `/Game/MetroidVania/Blueprints/Characters/BP_Player` Other))
  (`/Engine/EditorBlueprintResources/StandardMacros.DoOnce` false :!label _label
    (:`Completed`
      (`GameplayStatics.ApplyDamage` _asbp_player (`self.AttackDamage`))
      (`KismetSystemLibrary.Delay` 0.5)
      (goto _label :!via `Reset`))))

(fn `UserConstructionScript`)