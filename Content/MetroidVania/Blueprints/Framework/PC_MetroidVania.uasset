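; Player controller for the MetroidVania game that runs the black and white magic menus and the learned-skill popup.
; Both menus are created at BeginPlay and shown while their input is held, swapping out the HUD and pausing; release resumes play and animates any slotted selection.
; White magic requires the player's WMagicReady flag, with a Gate so release only closes a menu that opened.
; The skill popup pauses until dismissed by input.
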(event `ShowAcquiredSkill`
  (`GameplayStatics.SetGamePaused` true)
  (`UserWidget.AddToViewport` (`self.WBP_LearnedSkill`) 0))

(event `InputAction|Exit Skill Acquire` :consume false :paused true
  (params (Key :type "Key Structure"))
  (bind _returnvalue (`GameplayStatics.GetPlayerController` 0))
  ;[1 1 1] Hide acquired skill widget blueprint
  (:`Pressed`
    (if (`GameplayStatics.IsGamePaused`)
      (bind _wbp_learnedskill (`self.WBP_LearnedSkill`)
        (:`then`
          (`Widget.RemoveFromParent` _wbp_learnedskill)
          (`GameplayStatics.SetGamePaused` false)
          (`WidgetBlueprintLibrary.SetInputMode_GameOnly` _returnvalue)
          (set `PlayerController.bShowMouseCursor` false _returnvalue))
        (:`else`)))))

(event `self.ReceiveBeginPlay`
  (`|ExecutionSequence`
    (:`then_0`
      (bind _returnvalue (`|CreateWidget` "/Game/MetroidVania/Widgets/WBP_BMagic_Menu.WBP_BMagic_Menu_C"))
      (set `self.WBP_BMagicMenu` _returnvalue))
    (:`then_1`
      (bind _returnvalue_2 (`|CreateWidget` "/Game/MetroidVania/Widgets/WBP_WMagic_Menu.WBP_WMagic_Menu_C"))
      (set `self.WBP_WMagicMenu` _returnvalue_2))))

(event `InputAction|Black Magic Menu` :paused true
  (params (Key :type "Key Structure"))
  (bind _returnvalue (`GameplayStatics.GetPlayerController` 0))
  (bind _wbp_bmagicmenu (`self.WBP_BMagicMenu`))
  (:`Pressed`
    (bind _asmv_hud (cast `/Game/MetroidVania/Blueprints/Framework/MV_HUD` (`self.GetHUD`)))
    (bind _wbp_hud (`/Game/MetroidVania/Blueprints/Framework/MV_HUD.WBP_HUD` _asmv_hud))
    (`Widget.RemoveFromParent` _wbp_hud)
    (`UserWidget.AddToViewport` _wbp_bmagicmenu 0)
    (`UserWidget.PlayAnimation` _wbp_bmagicmenu (`/Game/MetroidVania/Widgets/WBP_BMagic_Menu.BMagicMenuIntro` _wbp_bmagicmenu) 0.0 1 "Forward" 1.0 false)
    (`GameplayStatics.PlaySound2D` (`self.SFX_Menu_ON`) 1.0 1.0 0.0 null null)
    (`GameplayStatics.SetGamePaused` true)
    (`WidgetBlueprintLibrary.SetInputMode_GameAndUIEx` _returnvalue (`self.WBP_BMagicMenu`)))
  (:`Released`
    (`UserWidget.AddToViewport` _wbp_hud 0)
    (`Widget.RemoveFromParent` _wbp_bmagicmenu)
    (`GameplayStatics.PlaySound2D` (`self.SFX_Menu_OFF`) 1.0 1.0 0.0 null null)
    (`GameplayStatics.SetGamePaused` false)
    (`WidgetBlueprintLibrary.SetInputMode_GameOnly` _returnvalue)
    (if (`/Game/MetroidVania/Widgets/WBP_BMagic_Menu.bSelectionMade?` (`self.WBP_BMagicMenu`))
      (`GameplayStatics.PlaySound2D` (`self.SFX_MagicSlotted`) 1.0 1.0 0.0 null null)
      (bind _asmv_hud_2 (cast `/Game/MetroidVania/Blueprints/Framework/MV_HUD` (`self.GetHUD`)))
      (bind _wbp_hud_2 (`/Game/MetroidVania/Blueprints/Framework/MV_HUD.WBP_HUD` _asmv_hud_2))
      (`UserWidget.PlayAnimation` _wbp_hud_2 (`/Game/MetroidVania/Widgets/WBP_HUD.BMagicSlotted` _wbp_hud_2) 0.0 1 "Forward" 1.0 false))))

(event `InputAction|White Magic Menu` :paused true
  (params (Key :type "Key Structure"))
  (bind _returnvalue (`GameplayStatics.GetPlayerController` 0))
  (bind _wbp_wmagicmenu (`self.WBP_WMagicMenu`))
  (:`Pressed`
    (bind _asbp_player (cast `/Game/MetroidVania/Blueprints/Characters/BP_Player` (`GameplayStatics.GetPlayerCharacter` 0)))
    (if (`/Game/MetroidVania/Blueprints/Characters/BP_Player.bWMagicReady?` _asbp_player)
      (`|ExecutionSequence`
        (:`then_0`
          (bind _asmv_hud (cast `/Game/MetroidVania/Blueprints/Framework/MV_HUD` (`self.GetHUD`)))
          (bind _wbp_hud (`/Game/MetroidVania/Blueprints/Framework/MV_HUD.WBP_HUD` _asmv_hud))
          (`Widget.RemoveFromParent` _wbp_hud)
          (`UserWidget.AddToViewport` _wbp_wmagicmenu 0)
          (`UserWidget.PlayAnimation` _wbp_wmagicmenu (`/Game/MetroidVania/Widgets/WBP_WMagic_Menu.WMagicMenuIntro` _wbp_wmagicmenu) 0.0 1 "Forward" 1.0 false)
          (`GameplayStatics.PlaySound2D` (`self.SFX_Menu_ON`) 1.0 1.0 0.0 null null)
          (`GameplayStatics.SetGamePaused` true)
          (`WidgetBlueprintLibrary.SetInputMode_GameAndUIEx` _returnvalue (`self.WBP_WMagicMenu`)))
        (:`then_1`
          (goto _label :!via `Open`)))
      (else
        (`GameplayStatics.PlaySound2D` (`self.SFX_ActionDisallowed`) 0.3 1.0 0.0 null null))))
  (:`Released`
    (`/Engine/EditorBlueprintResources/StandardMacros.Gate` true :!label _label
      (:`Exit`
        (`|ExecutionSequence`
          (:`then_0`
            (`UserWidget.AddToViewport` _wbp_hud 0)
            (`Widget.RemoveFromParent` _wbp_wmagicmenu)
            (`GameplayStatics.PlaySound2D` (`self.SFX_Menu_OFF`) 1.0 1.0 0.0 null null)
            (`GameplayStatics.SetGamePaused` false)
            (`WidgetBlueprintLibrary.SetInputMode_GameOnly` _returnvalue)
            (if (`/Game/MetroidVania/Widgets/WBP_WMagic_Menu.bSelectionMade?` (`self.WBP_WMagicMenu`))
              (`GameplayStatics.PlaySound2D` (`self.SFX_MagicSlotted`) 1.0 1.0 0.0 null null)
              (bind _asmv_hud_2 (cast `/Game/MetroidVania/Blueprints/Framework/MV_HUD` (`self.GetHUD`)))
              (bind _wbp_hud_2 (`/Game/MetroidVania/Blueprints/Framework/MV_HUD.WBP_HUD` _asmv_hud_2))
              (`UserWidget.PlayAnimation` _wbp_hud_2 (`/Game/MetroidVania/Widgets/WBP_HUD.WMagicSlotted` _wbp_hud_2) 0.0 1 "Forward" 1.0 false)))
          (:`then_1`
            (goto _label :!via `Close`)))))))

(fn `UserConstructionScript`)