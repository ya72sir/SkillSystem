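; BP_MistGate is a gate actor that tells the player when mist is needed.
; Overlapping its InteractCollider while not using mist shows WBPNotifier with the interact message, an intro animation and a sound.
; Leaving the collider or receiving the player's RemoveNeedMistMessage dispatcher reverses the animation, then removes the widget after a matching delay.
; BeginPlay runs the parent logic before binding that dispatcher.
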(event `self.ReceiveBeginPlay`
  ;[1 1 1] Subscribe to !remove Need Mist Message!
  (`|ExecutionSequence`
    (:`then_0`
      (`parent.ReceiveBeginPlay`))
    (:`then_1`
      (add `/Game/MetroidVania/Blueprints/Characters/BP_Player.RemoveNeedMistMessage` (`self.BP_Player`) (delegate `RemoveNeedMistMessage_Event_0`)))))

(event `RemoveNeedMistMessage_Event_0`
  ;[1 1 1] Subscribe to !remove Need Mist Message!
  (`self.RemoveMessage`))

(event `self.InteractCollider.OnComponentBeginOverlap`
  (params (OverlappedComponent :type "PrimitiveComponent Object Reference") (OtherActor :type "Actor Object Reference") (OtherComp :type "PrimitiveComponent Object Reference") (OtherBodyIndex :type Integer) (bFromSweep :type Boolean) (SweepResult :type "HitResult Structure (by ref)"))
  (bind _wbp_notifier (`self.WBP_Notifier`))
  (cast `/Game/MetroidVania/Blueprints/Characters/BP_Player` OtherActor)
  (if (not (`/Game/MetroidVania/Blueprints/Characters/BP_Player.bIsUsingMist?` (`self.BP_Player`)))
    (set `/Game/MetroidVania/Widgets/WBP_Notify.RecievedMessage` (`self.InteractMessage`) _wbp_notifier)
    (`UserWidget.AddToViewport` _wbp_notifier 0)
    (`UserWidget.PlayAnimation` _wbp_notifier (`/Game/MetroidVania/Widgets/WBP_Notify.Intro_NoButton` _wbp_notifier) 0.0 1 "Forward" 1.0 false)
    (`GameplayStatics.PlaySound2D` (`self.SFX_CanInteract`) 2.5 1.0 0.0 null null)))

(event `RemoveMessage`
  (bind _wbp_notifier (`self.WBP_Notifier`))
  (bind _intro_nobutton (`/Game/MetroidVania/Widgets/WBP_Notify.Intro_NoButton` _wbp_notifier))
  (`UserWidget.PlayAnimation` _wbp_notifier _intro_nobutton 0.0 1 "Reverse" 1.0 false :!label _label)
  (`KismetSystemLibrary.Delay` (`WidgetAnimation.GetEndTime` _intro_nobutton))
  (`Widget.RemoveFromParent` (`self.WBP_Notifier`)))

(event `self.InteractCollider.OnComponentEndOverlap`
  (params (OverlappedComponent :type "PrimitiveComponent Object Reference") (OtherActor :type "Actor Object Reference") (OtherComp :type "PrimitiveComponent Object Reference") (OtherBodyIndex :type Integer))
  (cast `/Game/MetroidVania/Blueprints/Characters/BP_Player` OtherActor)
  (goto _label))

(fn `UserConstructionScript`
  (`parent.UserConstructionScript`))