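; Interactable pickup that grants the player the WMagic Mist skill in the MetroidVania game.
; Overlapping its collider enables interaction and shows an animated notifier with sound if the player neither has nor is using Mist, then hides it on exit.
; Interacting sets the skill flags, plays a burst effect and destroys the pickup's components.
; After a short delay, it passes a skill-acquired widget to the player controller for display.
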(event `self.InteractCollider.OnComponentBeginOverlap`
  (params (OverlappedComponent :type "PrimitiveComponent Object Reference") (OtherActor :type "Actor Object Reference") (OtherComp :type "PrimitiveComponent Object Reference") (OtherBodyIndex :type Integer) (bFromSweep :type Boolean) (SweepResult :type "HitResult Structure (by ref)"))
  (bind _bp_player (`self.BP_Player`))
  (bind _wbp_notifier (`self.WBP_Notifier`))
  ;[1 1 1] ShowInteractMessage
  (bind _asbp_player (cast `/Game/MetroidVania/Blueprints/Characters/BP_Player` OtherActor))
  (set `/Game/MetroidVania/Blueprints/Characters/BP_Player.bCanInteract?` true _asbp_player)
  (if (`/Game/MetroidVania/Blueprints/Characters/BP_Player.bHasWMagicMist?` _bp_player)
    _
    (elif (not (`/Game/MetroidVania/Blueprints/Characters/BP_Player.bIsUsingMist?` _bp_player))
      (set `/Game/MetroidVania/Widgets/WBP_Notify.RecievedMessage` (`self.InteractMessage`) _wbp_notifier)
      (`UserWidget.AddToViewport` _wbp_notifier 0)
      (`UserWidget.PlayAnimation` _wbp_notifier (`/Game/MetroidVania/Widgets/WBP_Notify.Intro` _wbp_notifier) 0.0 1 "Forward" 1.0 false)
      (`GameplayStatics.PlaySound2D` (`self.SFX_CanInteract`) 5.0 1.0 0.0 null null))))

(event `self.InteractCollider.OnComponentEndOverlap`
  (params (OverlappedComponent :type "PrimitiveComponent Object Reference") (OtherActor :type "Actor Object Reference") (OtherComp :type "PrimitiveComponent Object Reference") (OtherBodyIndex :type Integer))
  (bind _wbp_notifier (`self.WBP_Notifier`))
  (bind _intro (`/Game/MetroidVania/Widgets/WBP_Notify.Intro` _wbp_notifier))
  (cast `/Game/MetroidVania/Blueprints/Characters/BP_Player` OtherActor)
  (`UserWidget.PlayAnimation` _wbp_notifier _intro 0.0 1 "Reverse" 1.0 false)
  (`KismetSystemLibrary.Delay` (`WidgetAnimation.GetEndTime` _intro))
  (`Widget.RemoveFromParent` (`self.WBP_Notifier`))
  (set `/Game/MetroidVania/Blueprints/Characters/BP_Player.bCanInteract?` false (`self.BP_Player`)))

(event `/Game/MetroidVania/Blueprints/Misc/BPI_Interact.ObjectInteractedWith`
  (bind _bp_player (`self.BP_Player`))
  (if (`/Game/MetroidVania/Blueprints/Characters/BP_Player.bHasWMagicMist?` _bp_player)
    (`KismetSystemLibrary.PrintString` "player already has mist")
    (else
      (set `/Game/MetroidVania/Blueprints/Characters/BP_Player.bHasWMagicMist?` true _bp_player)
      (set `/Game/MetroidVania/Blueprints/Characters/BP_Player.SkillAcquired` "NewEnumerator6" _bp_player)
      (`self.PlayerAcquiredSkillFX`)
      (`KismetSystemLibrary.Delay` 0.75)
      (bind _returnvalue (`|CreateWidget` "/Game/MetroidVania/Widgets/WBP_SkillAcquired.WBP_SkillAcquired_C"))
      (bind _aspc_metroid_vania (cast `/Game/MetroidVania/Blueprints/Framework/PC_MetroidVania` (`GameplayStatics.GetPlayerController` 0)))
      (set `/Game/MetroidVania/Blueprints/Framework/PC_MetroidVania.WBP_LearnedSkill` _returnvalue _aspc_metroid_vania)
      (`/Game/MetroidVania/Blueprints/Framework/PC_MetroidVania.ShowAcquiredSkill` _aspc_metroid_vania))))

(fn `PlayerAcquiredSkillFX`
  (`Widget.RemoveFromParent` (`self.WBP_Notifier`))
  (`GameplayStatics.SpawnEmitterAtLocation` "/Game/InfinityBladeEffects/Effects/FX_Treasure/Resources/P_OrePile_Explosion_Success.P_OrePile_Explosion_Success" (`SceneComponent.K2_GetComponentLocation` (`self.Skill_Mesh`)) (struct) (2.0 2.0 2.0))
  (`GameplayStatics.PlaySound2D` (`self.SFX_CanInteract`) 3.0 1.0 0.0 null null)
  (`ActorComponent.K2_DestroyComponent` (`self.Skill_Mesh`))
  (`ActorComponent.K2_DestroyComponent` (`self.Skill_VFX`))
  (`ActorComponent.K2_DestroyComponent` (`self.Skill_Light`))
  (`ActorComponent.K2_DestroyComponent` (`self.InteractCollider`)))

(fn `UserConstructionScript`
  (`parent.UserConstructionScript`))